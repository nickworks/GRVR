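; Spline-driven power line actor that builds a row of utility poles with cables strung between them, entirely in the construction script.
; A PowerPole child actor is added at each spline point, rotated to the spline, and stored in an array.
; A second pass snaps each pole's two cables to the next pole's connectors, setting length to connector distance plus random slack for varied sag.
; The last pole's cables get zero length.
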(fn `UserConstructionScript`
  (locals (NewLocalVar_0 :type "/Game/Version_1930s/PowerRailLines/PowerPole Object Reference"))
  (bind _indexofloop (`self.IndexOfLoop`))
  (bind _spline (`self.Spline`))
  (bind _output (`|GetArrayItem` (`self.AllChildActorsOfPowerline`) (`self.IndexLoop2`)))
  (bind _output_2 (`|GetArrayItem` (`self.AllChildActorsOfPowerline`) (`self.NumberSplinePoints`)))
  (bind _output_3 (`|GetArrayItem` (`self.AllChildActorsOfPowerline`) (+ (`self.IndexLoop2`) 1)))
  (bind _cable1 (`/Game/Version_1930s/PowerRailLines/PowerPole.Cable1` _output))
  (bind _cable2 (`/Game/Version_1930s/PowerRailLines/PowerPole.Cable2` _output))
  (bind _con1 (`/Game/Version_1930s/PowerRailLines/PowerPole.Con1` _output_3))
  (bind _con2 (`/Game/Version_1930s/PowerRailLines/PowerPole.Con2` _output_3))
  (bind _output_get (set `self.NumberSplinePoints` (- (`SplineComponent.GetNumberOfSplinePoints` (`self.Spline`)) 1)))
  (for _index (range (+ _output_get 1))
    (set `self.IndexOfLoop` _index)
    (bind _returnvalue (`AddComponent|NODE_AddChildActorComponent-0` :`RelativeTransform` (`KismetMathLibrary.Conv_VectorToTransform` (`SplineComponent.GetLocationAtSplinePoint` _spline _indexofloop "Local"))))
    (`ChildActorComponent.SetChildActorClass` _returnvalue "/Game/Version_1930s/PowerRailLines/PowerPole.PowerPole_C")
    (bind _aspower_pole (cast `/Game/Version_1930s/PowerRailLines/PowerPole` (`ChildActorComponent.ChildActor` _returnvalue)))
    (`KismetArrayLibrary.Array_Add` (`self.AllChildActorsOfPowerline`) _aspower_pole)
    (`SceneComponent.K2_SetRelativeRotation` _returnvalue (`SplineComponent.GetRotationAtSplinePoint` _spline _indexofloop "Local") false false))
  (for _index_2 (range (+ (`self.NumberSplinePoints`) 1))
    (set `self.IndexLoop2` _index_2)
    (`|ExecutionSequence`
      (:`then_0`
        (`SceneComponent.K2_AttachToComponent` _cable1 _con1 "None" "SnapToTarget" "SnapToTarget" "KeepWorld" true)
        (set `CableComponent.CableLength` (+ (`KismetMathLibrary.VSize` (- (`SceneComponent.K2_GetComponentLocation` (`/Game/Version_1930s/PowerRailLines/PowerPole.Con1` _output)) (`SceneComponent.K2_GetComponentLocation` _con1))) (`KismetMathLibrary.RandomFloatInRange` 0.0 50.0)) _cable1)
        (set `CableComponent.CableLength` 0.0 (`/Game/Version_1930s/PowerRailLines/PowerPole.Cable1` _output_2)))
      (:`then_1`
        (`SceneComponent.K2_AttachToComponent` _cable2 _con2 "None" "SnapToTarget" "SnapToTarget" "KeepWorld" true)
        (set `CableComponent.CableLength` (+ (`KismetMathLibrary.VSize` (- (`SceneComponent.K2_GetComponentLocation` (`/Game/Version_1930s/PowerRailLines/PowerPole.Con2` _output)) (`SceneComponent.K2_GetComponentLocation` _con2))) (`KismetMathLibrary.RandomFloatInRange` 0.0 50.0)) _cable2)
        (set `CableComponent.CableLength` 0.0 (`/Game/Version_1930s/PowerRailLines/PowerPole.Cable2` _output_2))))))